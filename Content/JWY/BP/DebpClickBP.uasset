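; DebpClickBP is a Blueprint that chooses which local scene to play for the Debp click location.
; PickLocalScene reads the Global_BP game instance, using MasterChoiceLog entry 8 to select the school (RS) or graveyard branch and Day parity to select its A or B variant.
; It never requests a travel prompt or breakdown skip.
; A first-meeting Bianca intro branch is left disconnected, and the events hold no active logic.
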(fn `PickLocalScene`
  (returns (SceneNickName :type String) (`AsktoTravel?` :type Boolean) (SkipBreakdown :type Boolean))
  (bind _asglobal_bp (cast `/Game/VN_Framework/Blueprints/Global_BP` (`GameplayStatics.GetGameInstance`)))
  ; 학교 선택지 선택했음
  (if (<= (`|GetArrayItem` (`/Game/VN_Framework/Blueprints/Global_BP.MasterChoiceLog` _asglobal_bp) 8) 3)
    (bind _returnvalue (== (mod (`/Game/VN_Framework/Blueprints/Global_BP.Day` _asglobal_bp) 2) 0))
    (if _returnvalue
      (return "Debp_RS_A" false false)
      (else
        (return "Debp_RS_B" false false)))
    (else
      ; 묘지 선택지 선택했음
      (if _returnvalue
        (return "Debp_Grave_A" false false)
        (else
          (return "Debp_Grave_B" false false))))))

(fn `UserConstructionScript`
  (`parent.UserConstructionScript`))