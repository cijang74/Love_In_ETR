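; BP_Cheat is an overlap-triggered actor meant to open Clear_Level, apparently as a cheat shortcut gated on player stats.
; On overlap it casts the game instance to Global_BP and checks that the first four StatLog entries exist.
; The following sum check adds literal zeros instead of StatLog values and compares the result to 40, so the level load never fires as written.
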(event `self.ReceiveActorBeginOverlap`
  (params (OtherActor :type "Actor Object Reference"))
  (bind _asglobal_bp (cast `/Game/VN_Framework/Blueprints/Global_BP` (`GameplayStatics.GetGameInstance`)))
  (bind _statlog (`/Game/VN_Framework/Blueprints/Global_BP.StatLog` _asglobal_bp))
  (if (and (`KismetArrayLibrary.Array_IsValidIndex` _statlog) (`KismetArrayLibrary.Array_IsValidIndex` _statlog 1) (`KismetArrayLibrary.Array_IsValidIndex` _statlog 2) (`KismetArrayLibrary.Array_IsValidIndex` _statlog 3))
    (if (== 40 (+ (+ 0 0) (+ 0 0)))
      (`GameplayStatics.OpenLevel` "Clear_Level"))))

(fn `UserConstructionScript`)